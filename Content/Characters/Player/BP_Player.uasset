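; Player character Blueprint that drives footstep audio from the movement state.
; BeginPlay starts a single auto-playing 2D Footsteps event, zeroes its parameter and stores the instance.
; UpdateMovement maps Idle, Walking and Sprinting to values of that parameter, so one persistent instance follows the state rather than triggering a sound per step.
; A StopMovementImmediately call is left unwired and never runs.
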(event EventBeginPlay
  (bind _returnvalue (Class|FMODBlueprintStatics|PlayEvent2D "/Game/FMOD/Events/SFX/Footsteps.Footsteps"))
  (Class|FMODBlueprintStatics|EventInstanceSetParameter _returnvalue "Footsteps" 0.0)
  (Variables|Default|SetFootsteps _returnvalue))

(event EventUpdateMovement
  (params (State :type EMovementState%20Enum%20%28by%20ref%29 :default "Idle"))
  (bind _footsteps (Variables|Default|GetFootsteps))
  (switch Utilities|FlowControl|Switch|SwitchonEMovementState State
    (:Idle
      (Class|FMODBlueprintStatics|EventInstanceSetParameter _footsteps "Footsteps" 0.0))
    (:Walking
      (Class|FMODBlueprintStatics|EventInstanceSetParameter _footsteps "Footsteps" 1.0))
    (:Sprinting
      (Class|FMODBlueprintStatics|EventInstanceSetParameter _footsteps "Footsteps" 2.0))))

(fn ConstructionScript)