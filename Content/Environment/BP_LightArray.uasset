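; BP_LightArray is an environment actor that lays out a configurable grid of child actors, named as lights, at construction.
; The Construction Script loops over the X by Y light count and adds a Child Actor Component per cell.
; A single index becomes column and row through modulo and integer division, scaled by per-axis spacing for relative location.
; The Event Graph holds only disabled default events, so it adds no runtime logic.
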(event EventBeginPlay)

(event Collision|EventActorBeginOverlap
  (params (OtherActor :type Actor%20Object%20Reference)))

(event EventTick
  (params (DeltaSeconds :type Float%20%28single-precision%29)))

(fn ConstructionScript
  (bind _numlightsx (Variables|Default|GetNumLightsX))
  (for _index (range 0 (- (* (Variables|Default|GetNumLightsX) (Variables|Default|GetNumLightsY)) 1))
    (AddComponent|AddChildActorComponent false (Math|Transform|MakeTransform (Math|Vector|MakeVector (* (Math|Integer|%(Integer) _index _numlightsx) (Variables|Default|GetLightSpacingX)) (* (/ _index _numlightsx) (Variables|Default|GetLightSpacingY)) 0.0) "0, 0, 0" "1.000000,1.000000,1.000000"))))