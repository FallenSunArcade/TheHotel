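; Robot prop that wakes up with flashing lights and an FMOD sound event while the player is inside its trigger box.
; Box overlaps switch it on or off after a delay, starting or stopping the sound.
; Tick, enabled only while on, blinks eye and headlight emission at a set interval through dynamic material instances created in the Construction Script.
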(event OnComponentEndOverlap(Box)
  (params (OverlappedComponent :type Primitive%20Component%20Object%20Reference) (OtherActor :type Actor%20Object%20Reference) (OtherComp :type Primitive%20Component%20Object%20Reference) (OtherBodyIndex :type Integer))
  ;[1 0.2188 0.2188] Triggers
  (Utilities|Casting|CastToBP_Player OtherActor)
  (Utilities|FlowControl|Delay (Variables|Default|GetTurnOffDelay))
  (CallFunction|TurnOff)
  (Class|FMODBlueprintStatics|EventInstanceStop (stale OnComponentBeginOverlap(Box) _returnvalue) false))

(event OnComponentBeginOverlap(Box)
  (params (OverlappedComponent :type Primitive%20Component%20Object%20Reference) (OtherActor :type Actor%20Object%20Reference) (OtherComp :type Primitive%20Component%20Object%20Reference) (OtherBodyIndex :type Integer) (bFromSweep :type Boolean) (SweepResult :type Hit%20Result%20Structure%20%28by%20ref%29))
  ;[1 0.2188 0.2188] Triggers
  (Utilities|Casting|CastToBP_Player OtherActor)
  (Utilities|FlowControl|Delay (Variables|Default|GetTurnOnDelay))
  (CallFunction|Turnon)
  (bind _returnvalue (Class|FMODBlueprintStatics|PlayEventatLocation "/Game/FMOD/Events/SFX/Robot.Robot" (Transformation|GetWorldTransform (Variables|Default|GetRobotMesh)))))

(event Custom|TurnOn
  ;[1 1 1] Turning On/Off Events
  (Actor|Tick|SetActorTickEnabled true)
  (Variables|Default|SetLightFlashElapsed 0.0)
  (Rendering|Material|SetScalarParameterValue (Variables|Default|GetEyesMaterial) "EmissionStrength" (Variables|Default|GetEyeBrightness) :!class /Script/Engine.MaterialInstanceDynamic)
  (Rendering|Material|SetScalarParameterValue (Variables|Default|GetHeadLightMaterial) "EmissionStrength" (Variables|Default|GetHeadLightBrightness) :!class /Script/Engine.MaterialInstanceDynamic))

(event Custom|TurnOff
  ;[1 1 1] Turning On/Off Events
  (Actor|Tick|SetActorTickEnabled false)
  (Rendering|Material|SetScalarParameterValue (Variables|Default|GetEyesMaterial) "EmissionStrength" 0.0 :!class /Script/Engine.MaterialInstanceDynamic)
  (Rendering|Material|SetScalarParameterValue (Variables|Default|GetHeadLightMaterial) "EmissionStrength" 0.0 :!class /Script/Engine.MaterialInstanceDynamic))

(event EventBeginPlay
  (CallFunction|TurnOff))

(event EventTick
  (params (DeltaSeconds :type Float%20%28single-precision%29))
  ;[1 0.9244 0.4436] Flicker
  (bind _output_get (Variables|Default|SetLightFlashElapsed (+ DeltaSeconds (Variables|Default|GetLightFlashElapsed))))
  (if (>= _output_get (Variables|Default|GetLightFlashInterval))
    (Variables|Default|SetLightFlashElapsed 0.0)
    (bind _returnvalue (Rendering|Material|GetScalarParameterValue (Variables|Default|GetEyesMaterial) "EmissionStrength" :!class /Script/Engine.MaterialInstanceDynamic))
    (if (== _returnvalue 0.0)
      (Rendering|Material|SetScalarParameterValue (Variables|Default|GetEyesMaterial) "EmissionStrength" (Variables|Default|GetEyeBrightness) :!class /Script/Engine.MaterialInstanceDynamic)
      (Rendering|Material|SetScalarParameterValue (Variables|Default|GetHeadLightMaterial) "EmissionStrength" (Variables|Default|GetHeadLightBrightness) :!class /Script/Engine.MaterialInstanceDynamic)
      (else
        (Rendering|Material|SetScalarParameterValue (Variables|Default|GetEyesMaterial) "EmissionStrength" 0.0 :!class /Script/Engine.MaterialInstanceDynamic)
        (Rendering|Material|SetScalarParameterValue (Variables|Default|GetHeadLightMaterial) "EmissionStrength" 0.0 :!class /Script/Engine.MaterialInstanceDynamic)))))

(fn ConstructionScript
  (bind _returnvalue (Rendering|Material|CreateDynamicMaterialInstance (Variables|Default|GetRobotMesh) 2 "/Game/Environment/Props/Materials/MI_RobotEyes.MI_RobotEyes" "None" :!class /Script/Engine.PrimitiveComponent))
  (Variables|Default|SetEyesMaterial _returnvalue)
  (bind _returnvalue_2 (Rendering|Material|CreateDynamicMaterialInstance (Variables|Default|GetRobotMesh) 3 "/Game/Environment/Props/Materials/MI_RobotHeadLight.MI_RobotHeadLight" "None" :!class /Script/Engine.PrimitiveComponent))
  (Variables|Default|SetHeadLightMaterial _returnvalue_2))