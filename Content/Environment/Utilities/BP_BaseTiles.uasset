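; BP_BaseTiles is a utility Blueprint that builds a rectangular grid of optional floor and ceiling tiles for environments.
; The construction script loops over every cell in the GridSizeX by GridSizeY grid, adding mesh instances to FloorMesh and CeilingMesh when enabled.
; CalculateGridLocation supplies each instance's X and Y from its index, with modulo and division scaled by TileSize.
; Ceiling instances are raised to CeilingHeight.
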(event EventBeginPlay)

(fn ConstructionScript
  (Variables|Default|SetLastIndex (- (* (Variables|Default|GetGridSizeX) (Variables|Default|GetGridSizeY)) 1))
  (Utilities|FlowControl|Sequence
    (:then_0
      (if (Variables|Default|GetCeiling)
        (for _index (range 0 (Variables|Default|GetLastIndex))
          (Components|InstancedStaticMesh|AddInstance (Variables|Default|GetCeilingMesh) (Math|Transform|MakeTransform (Math|Vector|MakeVector (.XLocation (Utilities|CalculateGridLocation _index)) (.YLocation (Utilities|CalculateGridLocation _index)) (Variables|Default|GetCeilingHeight)) "0, 0, 0" "1.000000,1.000000,1.000000") false))))
    (:then_1
      (if (Variables|Default|GetFloor)
        (for _index_2 (range 0 (Variables|Default|GetLastIndex))
          (Components|InstancedStaticMesh|AddInstance (Variables|Default|GetFloorMesh) (Math|Transform|MakeTransform (Math|Vector|MakeVector (.XLocation (Utilities|CalculateGridLocation _index_2)) (.YLocation (Utilities|CalculateGridLocation _index_2)) 0.0) "0, 0, 0" "1.000000,1.000000,1.000000") false))))))